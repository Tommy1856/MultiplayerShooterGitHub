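; Corridor door Blueprint that opens and closes only for players of a required rank.
; On Interact with either of two components, it checks the instigator's MyCurrentRank and prints a granted or denied message.
; A FlipFlop alternately plays and reverses the DoorControl timeline on each granted use.
; Tick only prints debug values of the timeline scaled by ±200; no door movement is wired here.
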(event `self.ReceiveTick`
  (params (DeltaSeconds :type "Float (single-precision)"))
  (`KismetSystemLibrary.PrintString` (`KismetStringLibrary.Conv_DoubleToString` (* (stale `/Game/Character/BlueprintInterface/Interact.Interact` _doorcontrol) 200.0)) true true (struct :`R` 0.038946 :`B` 1.0 :`A` 1.0) 0.0)
  (`KismetSystemLibrary.PrintString` (`KismetStringLibrary.Conv_DoubleToString` (* (stale `/Game/Character/BlueprintInterface/Interact.Interact` _doorcontrol) -200.0)) true true (struct :`R` 1.0 :`B` 0.113355 :`A` 1.0) 0.0))

(event `/Game/Character/BlueprintInterface/Interact.Interact`
  (params (Instigator :type "/Game/Character/BaseCharacter Object Reference") (Component :type "ActorComponent Object Reference") (HitActor :type "Actor Object Reference"))
  (if (or (== Component null) (== Component null))
    (if (`|EnumEquality` (`/Game/Character/BaseCharacter.My Current Rank` Instigator) "NewEnumerator8")
      (`KismetSystemLibrary.PrintString` "Access Granted" true true (struct :`G` 1.0 :`A` 1.0) 10.0)
      (`/Engine/EditorBlueprintResources/StandardMacros.FlipFlop`
        (:`A`
          (bind (_direction _doorcontrol) (`Timeline|DoorControl` :!label _label)))
        (:`B`
          (goto _label :!via `Reverse`)))
      (else
        (`KismetSystemLibrary.PrintString` "Access Denied: Rank too low" true true (struct :`R` 1.0 :`A` 1.0) 10.0)))))

(fn `Player to Player Interact Menu`
  (returns (Rank :type "/Game/Character/CloneRanks Enum"))
  (return "NewEnumerator0"))

(fn `UserConstructionScript`)